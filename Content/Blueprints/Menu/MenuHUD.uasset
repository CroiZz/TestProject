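; MenuHUD is the menu's HUD, showing the player's money and a loading image.
; Each DrawHUD call creates and adds a new MenuWidget to the viewport, then scales canvas drawing to screen width against a 640-pixel base.
; DrawMoney prints the score money read from InvaderInstance.
; A Now Loading texture is drawn while IsLoading is set.
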(event EventDrawHUD
  (params (SizeX :type Integer) (SizeY :type Integer))
  (bind _returnvalue (UserInterface|CreateWidget "/Game/Blueprints/Menu/MenuWidget.MenuWidget_C"))
  (Variables|Default|SetMenuWidget _returnvalue)
  (UserInterface|Viewport|AddtoViewport _returnvalue 0)
  (Variables|Default|SetScale (/ (Math|Conversions|ToFloat(Integer) SizeX) 6.4e+02))
  (CallFunction|DrawMoney "(X=0.000000,Y=200.000000)" (Variables|Default|GetScale))
  (if (Variables|Default|GetisLoading)
    (Canvas|DrawTexture "/Game/StarterContent/Textures/T_Nowloading.T_Nowloading" 0.0 (/ (- (Math|Conversions|ToFloat(Integer) SizeY) (* 3.6e+02 (Variables|Default|GetScale))) 2.0) 3.2e+02 64.0 0.0 0.0 1.0 1.0 "(R=1.000000,G=0.977639,B=0.987540,A=1.000000)" "BLEND_Translucent" (Variables|Default|GetScale))))

(fn ConstructionScript)

(fn DrawMoney
  (params (InPosition :type Vector%202D%20Structure) (InScale :type Float%20%28single-precision%29))
  (bind (_x _y) (Math|Vector2D|BreakVector2D InPosition))
  (bind _asinvader_instance (Utilities|Casting|CastToInvaderInstance (Game|GetGameInstance)))
  (bind _scoremoney (Default|GetScoreMoney _asinvader_instance))
  (HUD|DrawText (Utilities|String|BuildString(Integer) "" "Money:" _scoremoney) "(R=0,G=0,B=0,A=1)" _x _y 0 InScale true))