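; Title screen HUD that draws the title image with Start and End buttons.
; DrawHUD scales a 640x360 layout to the screen width, centers it vertically, and lays invisible hit boxes over the button areas.
; Clicking Start sets IsLoading to swap in a Now Loading texture, calls LoadStreamLevel on Menu, then immediately opens that level.
; Clicking End quits the game.
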(event EventDrawHUD
  (params (SizeX :type Integer) (SizeY :type Integer))
  ;[1 1 1] タイトル画面を描画
  (Variables|Default|SetScale (/ (Math|Conversions|ToFloat(Integer) SizeX) 6.4e+02))
  ;[1 1 1] Startボタンが押されたか？
  (if (Variables|Default|GetIsLoading)
    ;[1 1 1] NowLoading表示
    (Canvas|DrawTexture "/Game/StarterContent/Textures/T_Nowloading.T_Nowloading" 0.0 (/ (- (Math|Conversions|ToFloat(Integer) SizeY) (* 3.6e+02 (Variables|Default|GetScale))) 2.0) 3.2e+02 64.0 0.0 0.0 1.0 1.0 "(R=1.000000,G=1.000000,B=1.000000,A=1.000000)" "BLEND_Translucent" (Variables|Default|GetScale))
    (else
      (Canvas|DrawTexture "/Game/StarterContent/Textures/T_Title.T_Title" 0.0 (/ (- (Math|Conversions|ToFloat(Integer) SizeY) (* 3.6e+02 (Variables|Default|GetScale))) 2.0) 6.4e+02 3.6e+02 0.0 0.0 1.0 1.0 "(R=1.000000,G=1.000000,B=1.000000,A=1.000000)" "BLEND_Translucent" (Variables|Default|GetScale))
      ;[1 1 1] ボタン追加
      (Class|HUD|AddHitBox (+ (* (Math|Vector2D|MakeVector2D 23.0 214.0) (Variables|Default|GetScale)) (Math|Vector2D|MakeVector2D 0.0 (/ (- (Math|Conversions|ToFloat(Integer) SizeY) (* 3.6e+02 (Variables|Default|GetScale))) 2.0))) (* (Math|Vector2D|MakeVector2D 2.5e+02 58.0) (Variables|Default|GetScale)) "Start" false)
      (Class|HUD|AddHitBox (+ (Math|Vector2D|MakeVector2D 0.0 (/ (- (Math|Conversions|ToFloat(Integer) SizeY) (* 3.6e+02 (Variables|Default|GetScale))) 2.0)) (* (Math|Vector2D|MakeVector2D 23.0 2.8e+02) (Variables|Default|GetScale))) (* (Math|Vector2D|MakeVector2D 2.5e+02 58.0) (Variables|Default|GetScale)) "End" false))))

(event EventHitBoxClick
  (params (BoxName :type Name))
  ;[1 1 1] シーン遷移
  (switch name BoxName
    (:Start
      (Variables|Default|SetIsLoading true)
      (Game|LoadStreamLevel(byName) "Menu" false)
      (Game|OpenLevel(byName) "Menu"))
    (:End
      (Game|QuitGame 0 "Quit"))))

(fn ConstructionScript)