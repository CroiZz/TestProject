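; InvaderInstance is a Game Instance Blueprint that holds the player's bullet damage and score money for an invader game.
; Each value has a getter and an add function that increases it by the passed amount.
; As game instance state, both values persist across level loads; the file contains no save, reset or clamping logic.
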(fn GetPlayerBulletDamage
  (return (Variables|Default|GetPlayerBulletDamage)))

(fn AddPlayerBulletDamage
  (params (AddDamage :type Integer))
  (Variables|Default|SetPlayerBulletDamage (+ AddDamage (Variables|Default|GetPlayerBulletDamage))))

(fn GetScoreMoney
  (return (Variables|Default|GetScoreMoney)))

(fn AddScoreMoney
  (params (ScoreMoney :type Integer))
  (Variables|Default|SetScoreMoney (+ ScoreMoney (Variables|Default|GetScoreMoney))))