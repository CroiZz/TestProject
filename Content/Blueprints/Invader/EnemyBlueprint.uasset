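; Invader enemy actor that slides sideways, fires bullets and awards score when killed.
; Each tick it moves along Y using the GameState's shared DirectionY and counts down a randomized timer that spawns EnemyBulletBlueprint just below it.
; Damage lowers Health; at zero it spawns an explosion, adds score to GameState and InvaderInstance, then destroys itself.
; The bullet overlap handler only casts, and the player health and score getters return zero.
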(event EventTick
  (params (DeltaSeconds :type Float%20%28single-precision%29))
  ;[1 1 1] 移動
  (bind _asmy_game_state (Utilities|Casting|CastToMyGameState (Game|GetGameState)))
  (Transformation|SetActorLocation (+ (* (* "0,1.000000, 0" (Variables|/Game/Blueprints/Invader/MyGameState.MyGameState_C|GetDirectionY _asmy_game_state)) (* "0,50.000000, 0" DeltaSeconds)) (Transformation|GetActorLocation)) false false)
  (CallFunction|ShotBullet DeltaSeconds))

(event Collision|EventActorBeginOverlap
  (params (OtherActor :type Actor%20Object%20Reference))
  ;[1 1 1] 爆発処理
  (Utilities|Casting|CastToPlayerBulletBlueprint OtherActor))

(event Game|Damage|EventAnyDamage
  (params (Damage :type Float%20%28single-precision%29) (DamageType :type Damage%20Type%20Object%20Reference) (InstigatedBy :type Controller%20Object%20Reference) (DamageCauser :type Actor%20Object%20Reference))
  ;[1 1 1] ダメージ計算
  (bind _output_get (Variables|Default|SetHealth (- (Variables|Default|GetHealth) (Math|Float|Floor Damage))))
  ;[1 1 1] 爆発処理
  (if (<= _output_get 0)
    (Game|SpawnActorfromClass "/Game/StarterContent/Blueprints/Blueprint_Effect_Explosion.Blueprint_Effect_Explosion_C" (Math|Conversions|ToTransform(Vector) (Transformation|GetActorLocation)) "Undefined" 0 0)
    ;[1 1 1] スコア加算
    (Class|MyInterface|AddScore(Message) (Game|GetGameState) 10)
    (bind _asinvader_instance (Utilities|Casting|CastToInvaderInstance (Game|GetGameInstance)))
    (Default|AddScoreMoney _asinvader_instance 10)
    (Actor|DestroyActor)))

(fn ConstructionScript
  (Variables|Default|SetShotTimer (Math|Random|RandomFloatinRange 1.0 1e+01)))

(fn ShotBullet
  (params (DeltaTime :type Float%20%28single-precision%29))
  (if (< (- (Variables|Default|GetShotTimer) DeltaTime) 0.0)
    (Game|SpawnActorfromClass "/Game/Blueprints/Invader/EnemyBulletBlueprint.EnemyBulletBlueprint_C" (Math|Conversions|ToTransform(Vector) (+ (Transformation|GetActorLocation) "0, 0,-40.000000")) "Undefined" 0 0)
    (Variables|Default|SetShotTimer (Math|Random|RandomFloatinRange 1.0 1e+01))
    (else
      (Variables|Default|SetShotTimer (- (Variables|Default|GetShotTimer) DeltaTime))))
  (return))

(fn GetEnemyHealth
  (return (Variables|Default|GetHealth)))

(fn GetPlayerHealth
  (return 0))

(fn GetScore
  (return 0))