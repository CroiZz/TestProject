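; Player Blueprint for an Invader shooter: a ship that slides along the Y axis with mouse X and fires bullets on left click.
; Damage reduces Health; at zero it spawns an explosion, then hides itself and disables collision.
; The hidden state doubles as the death flag, blocking movement and turning left click into a return to the Title level.
; Getters expose Health and the hidden flag, while enemy health and score getters are stubs returning zero.
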(event Game|Damage|EventAnyDamage
  (params (Damage :type Float%20%28single-precision%29) (DamageType :type Damage%20Type%20Object%20Reference) (InstigatedBy :type Controller%20Object%20Reference) (DamageCauser :type Actor%20Object%20Reference))
  ;[1 1 1] ダメージ処理
  (bind _output_get (Variables|Default|SetHealth (- (Variables|Default|GetHealth) (Math|Float|Floor Damage))))
  ;[1 1 1] 死亡処理
  (if (<= _output_get 0)
    (Game|SpawnActorfromClass "/Game/StarterContent/Blueprints/Blueprint_Effect_Explosion.Blueprint_Effect_Explosion_C" (Math|Conversions|ToTransform(Vector) (Transformation|GetActorLocation)) "Undefined" 0 0)
    (Rendering|SetActorHiddenInGame true)
    (Collision|SetActorEnableCollision false)))

(event Input|MouseEvents|MouseX
  (params (AxisValue :type Float%20%28single-precision%29))
  ;[1 1 1] 移動
  (if (not (Variables|Rendering|GetbHidden))
    (Transformation|SetActorLocation (+ (* "0,10.000000, 0" AxisValue) (Transformation|GetActorLocation)) false false)))

(event Input|MouseEvents|LeftMouseButton
  (params (Key :type Key%20Structure :default "AnyKey"))
  ;[1 1 1] 弾の発射
  (:Pressed
    (if (Variables|Rendering|GetbHidden)
      ;[1 1 1] タイトルへ遷移
      (Game|OpenLevel(byName) "Title")
      (else
        (Game|SpawnActorfromClass "/Game/Blueprints/Invader/PlayerBulletBlueprint.PlayerBulletBlueprint_C" (Math|Conversions|ToTransform(Vector) (+ (Transformation|GetActorLocation) "0, 0,30.000000")) "Undefined" 0 0)))))

(fn ConstructionScript)

(fn GetHidePlayerFlg
  (return (Variables|Rendering|GetbHidden)))

(fn GetEnemyHealth
  (return 0))

(fn GetPlayerHealth
  (return (Variables|Default|GetHealth)))

(fn GetScore
  (return 0))