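; HUD for the Invader game that draws the score, the player's HP bar and text, and a Game Over image.
; DrawHUD reads the score from the GameState and health from the player pawn, showing Game Over when the pawn's hide flag is set.
; Elements scale by screen width against a 640-pixel base, and the bar crops its texture by health.
; The enemy HP helper is never called here, and three getters return zero.
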(event EventDrawHUD
  (params (SizeX :type Integer) (SizeY :type Integer))
  (bind _returnvalue (Math|Conversions|ToFloat(Integer) SizeX))
  (bind _returnvalue_2 (/ _returnvalue 6.4e+02))
  ;[1 1 1] 画面サイズに合わせる
  ;[1 1 1] スコア表示
  (bind _score (Class|MyInterface|GetScore(Message) (Game|GetGameState)))
  (HUD|DrawText (Utilities|String|BuildString(Integer) "" "SCORE:" _score) "(R=0.971716,G=0.978787,B=1.000000,A=1.000000)" 2e+01 1e+01 0 _returnvalue_2 true)
  ;[1 1 1] HP表示
  (CallFunction|DrawPlayerHealthBar "(X=490.000000,Y=15.000000)" _returnvalue_2)
  (CallFunction|DrawPlayerHealthText "(X=490.000000,Y=35.000000)" _returnvalue_2)
  ;[1 1 1] GameOver表示
  (bind _asplayer_blueprint (Utilities|Casting|CastToPlayerBlueprint (Game|Player|GetPlayerPawn 0)))
  (bind _ishide (Default|GetHidePlayerFlg _asplayer_blueprint))
  (if _ishide
    (Class|HUD|DrawTextureSimple "/Game/StarterContent/Textures/T_Gameover.T_Gameover" 1.2e+02 1.3e+02 _returnvalue_2 true)))

(fn ConstructionScript)

(fn DrawPlayerHealthBar
  (params (InPosition :type Vector%202D%20Structure) (InScale :type Float%20%28single-precision%29))
  (bind (_x _y) (Math|Vector2D|BreakVector2D InPosition))
  (bind _health (Class|MyInterface|GetPlayerHealth(Message) (Game|Player|GetPlayerPawn 0)))
  (Canvas|DrawTexture "/Game/StarterContent/Textures/T_HPbar.T_HPbar" _x _y (* (/ (Math|Conversions|ToFloat(Integer) _health) 1e+02) 128.0) 16.0 0.0 0.5 (/ (Math|Conversions|ToFloat(Integer) _health) 1e+02) 0.5 "(R=1.000000,G=1.000000,B=1.000000,A=1.000000)" "BLEND_Translucent" InScale true))

(fn DrawPlayerHealthText
  (params (InPosition :type Vector%202D%20Structure) (InScale :type Float%20%28single-precision%29))
  (bind (_x _y) (Math|Vector2D|BreakVector2D InPosition))
  (bind _health (Class|MyInterface|GetPlayerHealth(Message) (Game|Player|GetPlayerPawn 0)))
  (HUD|DrawText (Utilities|String|BuildString(Integer) "" "HP:" _health) "(R=1.000000,G=0.985858,B=0.943431,A=1.000000)" _x _y 0 InScale true))

(fn DrawEnemyHealthText
  (params (InPosition :type Vector%202D%20Structure) (InScale :type Float%20%28single-precision%29))
  (bind (_x _y) (Math|Vector2D|BreakVector2D InPosition))
  (bind _health (Class|MyInterface|GetEnemyHealth(Message) (Game|Player|GetPlayerPawn 0)))
  (HUD|DrawText (Utilities|String|BuildString(Integer) "" "HP:" _health) "(R=0,G=0,B=0,A=1)" _x _y 0 InScale true))

(fn GetEnemyHealth
  (return 0))

(fn GetPlayerHealth
  (return 0))

(fn GetScore
  (return 0))