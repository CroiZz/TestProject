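; BulletBlueprint is a bullet actor, filed under an Invader game, that moves by a supplied vector and removes itself at the screen edges.
; MoveBullet adds the Location input, scaled by DeltaTime, to the actor's position without sweeping, so Location acts as a velocity.
; It then destroys the actor once its Z passes fixed upper or lower bounds.
; The file contains no caller for MoveBullet, and its construction script is empty.
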(fn ConstructionScript)

(fn MoveBullet
  (params (Location :type Vector) (DeltaTime :type Float%20%28single-precision%29))
  (bind _returnvalue (Transformation|GetActorLocation))
  (bind _z (Math|Vector|BreakVector _returnvalue))
  ;[1 1 1] 移動
  (Transformation|SetActorLocation (+ (* Location DeltaTime) (Transformation|GetActorLocation)) false false)
  ;[1 1 1] 画面端で消える
  (if (> _z 1e+03)
    (Actor|DestroyActor)
    (elif (< _z -1e+03)
      (Actor|DestroyActor))))